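; DReyeVR ego vehicle Blueprint that adjusts its planar reflections and otherwise leans on its parent class.
; On BeginPlay, the center, left and right planar reflection components each hide the vehicle Mesh, keeping it out of those reflections.
; Overlap, Tick and construction only forward to the parent.
; A SetTimer function decrements a Timer variable by one, with no caller in this Blueprint.
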(event Collision|EventActorBeginOverlap
  (params (OtherActor :type Actor%20Object%20Reference))
  (|CallParentFunction OtherActor))

(event EventBeginPlay
  (bind _mesh (Variables|Character|GetMesh))
  (Class|SceneCaptureComponent|HideComponent (Variables|Default|GetPlanarReflection) _mesh)
  (Class|SceneCaptureComponent|HideComponent (Variables|Default|GetPlanarReflectionLeft) _mesh)
  (Class|SceneCaptureComponent|HideComponent (Variables|Default|GetPlanarReflectionRight) _mesh))

(event EventTick
  (params (DeltaSeconds :type Float%20%28single-precision%29))
  (|CallParentFunction DeltaSeconds))

(fn ConstructionScript
  (|CallParentFunction))

(fn SetTimer
  (Variables|Default|SetTimer (- (Variables|Default|GetTimer) 1)))